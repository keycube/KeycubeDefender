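; Game mode for the KCD game that wires up the level's key actors and hands the player control of the cube at BeginPlay.
; It caches the first KCD_Spawner and KCD_LaneHolder found as ShipSpawner and LaneHolder, then player controller 0 possesses the first BP_KCD_Cube.
; An unconnected alternative setup uses the multi-target spawner and cube, with validity warnings, but never runs.
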(event `self.ReceiveBeginPlay`
  (bind _outactors (`GameplayStatics.GetAllActorsOfClass` "/Script/KeycubeDefender.KCD_Spawner"))
  (set `self.ShipSpawner` (`|GetArrayItem` _outactors))
  (bind _outactors_2 (`GameplayStatics.GetAllActorsOfClass` "/Script/KeycubeDefender.KCD_LaneHolder"))
  (set `self.LaneHolder` (`|GetArrayItem` _outactors_2))
  (bind _outactors_3 (`GameplayStatics.GetAllActorsOfClass` "/Game/Game/Blueprints/Cube/BP_KCD_Cube.BP_KCD_Cube_C"))
  (`Controller.Possess` (`GameplayStatics.GetPlayerController` 0) (`|GetArrayItem` _outactors_3)))

(fn `UserConstructionScript`)