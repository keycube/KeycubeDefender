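; BP_Key is an actor that represents a single keyboard key as a cube with a letter label.
; On BeginPlay it sets the label to the display name of its associated key and creates a dynamic material instance from MI_BaseKey on the cube.
; Its KeyPressed and KeyReleased events switch the material's Color parameter between the pressed and default colors.
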(event `self.ReceiveBeginPlay`
  (`TextRenderComponent.K2_SetText` (`self.KeyLetter`) (`KismetInputLibrary.Key_GetDisplayName` (`self.AssociatedKey`)))
  (bind _returnvalue (`PrimitiveComponent.CreateDynamicMaterialInstance` (`self.Cube`) 0 "/Game/Game/Materials/MI_BaseKey.MI_BaseKey" "None"))
  (set `self.DynamicMat` _returnvalue))

(event `KeyPressed`
  (`MaterialInstanceDynamic.SetVectorParameterValue` (`self.DynamicMat`) "Color" (`self.PressedColor`)))

(event `KeyReleased`
  (`MaterialInstanceDynamic.SetVectorParameterValue` (`self.DynamicMat`) "Color" (`self.DefaultColor`)))

(fn `UserConstructionScript`)